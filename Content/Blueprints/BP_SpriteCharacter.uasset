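; Player 2D sprite character with walking, scaled vertical movement, Shift sprinting and an F-toggled thinking animation.
; Tick picks the walk or idle flipbook from velocity and flips the sprite through control rotation.
; Any capsule overlap divides camera arm length and sprite scale by a multiplier, restored on exit.
; For BP_HouseExterior overlaps it also hides the exterior mesh, lowers walk speed and changes post-process focus and vignette, reversing these on exit.
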(event `self.ReceiveTick`
  (params (DeltaSeconds :type "Float (single-precision)"))
  ;[1 1 1] Will be called every Frame
  ;;[1 1 1] Check if Animation needs to be changed
  (`self.UpdateAnimation`)
  ;;[1 1 1] Check if Player Sprite needs to be flipped
  (`self.UpdateControlRotation`))

(event `InputAction|Jump`
  (params (Key :type "Key Structure"))
  ;[1 1 1] Jump?
)

(event `InputAxis|MoveRight`
  (params (AxisValue :type "Float (single-precision)"))
  ;[1 1 1] Move
  (if (`self.isSprinting?`)
    (set `CharacterMovementComponent.MaxWalkSpeed` (* (`self.MaxWalkSpeed`) (`self.SprintSpeedMultiplier`)) (`self.CharacterMovement`))
    (else
      (set `CharacterMovementComponent.MaxWalkSpeed` (`self.MaxWalkSpeed`) (`self.CharacterMovement`))))
  (`self.AddMovementInput` (1.0 0.0 0.0) AxisValue))

(event `InputAxis|MoveUp`
  (params (AxisValue :type "Float (single-precision)"))
  ;[1 1 1] Move
  (`self.AddMovementInput` (0.0 -1.0 0.0) (* AxisValue (`self.VerticalMovementSpeedMultiplier`))))

(event `Key|LeftShift`
  (params (Key :type "Key Structure"))
  ;[1 1 1] Move
  (:`Pressed`
    (set `self.isSprinting?` true))
  (:`Released`
    (set `self.isSprinting?` false)))

(event `UpdateAnimation`
  (bind _sprite (`self.Sprite`))
  ;[1 1 1] Change Animation when running
  (if (> (`KismetMathLibrary.VSize` (`MovementComponent.Velocity` (`self.CharacterMovement`))) 0.0)
    (`PaperFlipbookComponent.SetFlipbook` _sprite "/Game/Assets/Sprites/Characters/Ku/WithNormals/walking/Ku_normals_walking.Ku_normals_walking")
    (set `self.isAbleToIdle?` true)
    (elif (`self.isAbleToIdle?`)
      (`PaperFlipbookComponent.SetFlipbook` _sprite "/Game/Assets/Sprites/Characters/Ku/WithNormals/idle/Ku_Normal_Idle.Ku_Normal_Idle"))))

(event `UpdateControlRotation`
  ;[1 1 1] Rotate Character to face the other side when walking in other direction
  (`/Engine/EditorBlueprintResources/StandardMacros.IsValid` (`self.GetController`)
    (:`Is Valid`
      (`/Engine/EditorBlueprintResources/StandardMacros.CompareFloat` (.x (`MovementComponent.Velocity` (`self.CharacterMovement`)))
        (:`>`
          (`Controller.SetControlRotation` (`self.GetController`) (`KismetMathLibrary.MakeRotator` 0.0 0.0 180.0)))
        (:`<`
          (`Controller.SetControlRotation` (`self.GetController`) (`KismetMathLibrary.MakeRotator` 0.0)))))))

(event `Key|F`
  (params (Key :type "Key Structure"))
  ;[1 1 1] Play Animation on F
  (:`Pressed`
    (if (`self.isAbleToIdle?`)
      (set `self.isAbleToIdle?` false)
      (else
        (set `self.isAbleToIdle?` true)))
    (`/Engine/EditorBlueprintResources/StandardMacros.IsValid` (`self.GetController`)
      (:`Is Valid`
        (`/Engine/EditorBlueprintResources/StandardMacros.CompareFloat` (.x (`MovementComponent.Velocity` (`self.CharacterMovement`)))
          (:`==`
            (`PaperFlipbookComponent.SetFlipbook` (`self.Sprite`) "/Game/Assets/Sprites/Characters/Ku/WithNormals/thinking/Ku_normals_thinking.Ku_normals_thinking")))))))

(event `self.CapsuleComponent.OnComponentBeginOverlap`
  (params (OverlappedComponent :type "PrimitiveComponent Object Reference") (OtherActor :type "Actor Object Reference") (OtherComp :type "PrimitiveComponent Object Reference") (OtherBodyIndex :type Integer) (bFromSweep :type Boolean) (SweepResult :type "HitResult Structure (by ref)"))
  (bind _springarm (`self.SpringArm`))
  (bind _sprite (`self.Sprite`))
  (bind ((`AutoExposureMethod` _autoexposuremethod) (`AmbientCubemapTint` _ambientcubemaptint) (`AmbientCubemapIntensity` _ambientcubemapintensity) (`AmbientCubemap` _ambientcubemap) (`DepthOfFieldFstop` _depthoffieldfstop) (`DepthOfFieldMinFstop` _depthoffieldminfstop) (`DepthOfFieldBladeCount` _depthoffieldbladecount) (`AutoExposureBias` _autoexposurebias) (`AutoExposureMaxBrightness` _autoexposuremaxbrightness) (`VignetteIntensity` _vignetteintensity) (`DepthOfFieldSensorWidth` _depthoffieldsensorwidth) (`DepthOfFieldSqueezeFactor` _depthoffieldsqueezefactor) (`DepthOfFieldFocalDistance` _depthoffieldfocaldistance) (`DepthOfFieldVignetteSize` _depthoffieldvignettesize)) (break `PostProcessSettings` (`CameraComponent.PostProcessSettings` (`self.Camera`))))
  ;[1 1 1] VISUAL CHANGES WHEN ENTERING HOUSE
  (`KismetSystemLibrary.PrintString` "Player ENTERED Trigger")
  ;;[1 1 1] Adjust Camera Distance
  (set `SpringArmComponent.TargetArmLength` (/ (`SpringArmComponent.TargetArmLength` _springarm) (`self.InBuildingPlayerAdjustmentsMultiplier`)) _springarm)
  ;;[1 1 1] Adjust Player Size
  (`SceneComponent.SetWorldScale3D` _sprite (/ (`SceneComponent.K2_GetComponentScale` _sprite) (`self.InBuildingPlayerAdjustmentsMultiplier`)))
  ;;[1 1 1] Slightly Offset Player Position (to adjust to the size change)
  (`SceneComponent.K2_AddLocalOffset` (`self.Sprite`) (0.0 0.0 -6.0) false false)
  ;;[1 1 1] Hide Objects
  (bind _asbp_house_exterior (cast `/Game/Blueprints/BP_HouseExterior` OtherActor)
    (:`then`
      (`StaticMeshComponent.SetStaticMesh` (`/Game/Blueprints/BP_HouseExterior.StaticMesh` _asbp_house_exterior) null)
      ;;[1 1 1] Adjust Post Process Settings
      (set `CameraComponent.PostProcessSettings` (make `PostProcessSettings` :`AutoExposureMethod` _autoexposuremethod :`AmbientCubemapTint` _ambientcubemaptint :`AmbientCubemapIntensity` _ambientcubemapintensity :`AmbientCubemap` _ambientcubemap :`DepthOfFieldFstop` _depthoffieldfstop :`DepthOfFieldMinFstop` _depthoffieldminfstop :`DepthOfFieldBladeCount` _depthoffieldbladecount :`AutoExposureBias` _autoexposurebias :`AutoExposureMaxBrightness` _autoexposuremaxbrightness :`VignetteIntensity` 0.75 :`DepthOfFieldSensorWidth` _depthoffieldsensorwidth :`DepthOfFieldSqueezeFactor` _depthoffieldsqueezefactor :`DepthOfFieldFocalDistance` 360.0 :`DepthOfFieldVignetteSize` _depthoffieldvignettesize) (`self.Camera`))
      ;;[1 1 1] Adjust Player Movementspeed
      (set `self.MaxWalkSpeed` (/ (`self.MaxWalkSpeed`) (`self.InBuildingPlayerAdjustmentsMultiplier`)))
      ;;;[1 0.5906 0.6308] Debug
      (`KismetSystemLibrary.PrintString` (`KismetStringLibrary.Concat_StrStr` "Movement Speed: " (`KismetStringLibrary.Conv_DoubleToString` (`self.MaxWalkSpeed`)))))
    (:`CastFailed`
      (`KismetSystemLibrary.PrintString` "Cast to BP_HouseExterior FAILED when trying to ENTER  the Trigger!"))))

(event `self.CapsuleComponent.OnComponentEndOverlap`
  (params (OverlappedComponent :type "PrimitiveComponent Object Reference") (OtherActor :type "Actor Object Reference") (OtherComp :type "PrimitiveComponent Object Reference") (OtherBodyIndex :type Integer))
  (bind _springarm (`self.SpringArm`))
  (bind _sprite (`self.Sprite`))
  (bind ((`AutoExposureMethod` _autoexposuremethod) (`AmbientCubemapTint` _ambientcubemaptint) (`AmbientCubemapIntensity` _ambientcubemapintensity) (`AmbientCubemap` _ambientcubemap) (`DepthOfFieldFstop` _depthoffieldfstop) (`DepthOfFieldMinFstop` _depthoffieldminfstop) (`DepthOfFieldBladeCount` _depthoffieldbladecount) (`AutoExposureBias` _autoexposurebias) (`AutoExposureMaxBrightness` _autoexposuremaxbrightness) (`VignetteIntensity` _vignetteintensity) (`DepthOfFieldSensorWidth` _depthoffieldsensorwidth) (`DepthOfFieldSqueezeFactor` _depthoffieldsqueezefactor) (`DepthOfFieldFocalDistance` _depthoffieldfocaldistance) (`DepthOfFieldVignetteSize` _depthoffieldvignettesize)) (break `PostProcessSettings` (`CameraComponent.PostProcessSettings` (`self.Camera`))))
  ;[1 1 1] VISUAL CHANGES WHEN ENTERING HOUSE
  (`KismetSystemLibrary.PrintString` "Player LEFT Trigger")
  ;;[1 1 1] Adjust Camera Distance
  (set `SpringArmComponent.TargetArmLength` (* (`SpringArmComponent.TargetArmLength` _springarm) (`self.InBuildingPlayerAdjustmentsMultiplier`)) _springarm)
  ;;[1 1 1] Adjust Player Size
  (`SceneComponent.SetWorldScale3D` _sprite (* (`self.InBuildingPlayerAdjustmentsMultiplier`) (`SceneComponent.K2_GetComponentScale` _sprite)))
  ;;[1 1 1] Slightly Offset Player Position (to adjust to the size change)
  (`SceneComponent.K2_AddLocalOffset` (`self.Sprite`) (0.0 0.0 6.0) false false)
  ;;[1 1 1] Hide Objects
  (bind _asbp_house_exterior (cast `/Game/Blueprints/BP_HouseExterior` OtherActor)
    (:`then`
      (`StaticMeshComponent.SetStaticMesh` (`/Game/Blueprints/BP_HouseExterior.StaticMesh` _asbp_house_exterior) "/Game/Assets/Meshes/House_Exterior.House_Exterior")
      ;;[1 1 1] Adjust Post Process Settings
      (set `CameraComponent.PostProcessSettings` (make `PostProcessSettings` :`AutoExposureMethod` _autoexposuremethod :`AmbientCubemapTint` _ambientcubemaptint :`AmbientCubemapIntensity` _ambientcubemapintensity :`AmbientCubemap` _ambientcubemap :`DepthOfFieldFstop` 1.2 :`DepthOfFieldMinFstop` 0.0 :`AutoExposureBias` _autoexposurebias :`AutoExposureMaxBrightness` _autoexposuremaxbrightness :`DepthOfFieldSensorWidth` 200.0 :`DepthOfFieldFocalDistance` 520.0 :`DepthOfFieldVignetteSize` _depthoffieldvignettesize) (`self.Camera`))
      ;;[1 1 1] Adjust Player Movementspeed
      (set `self.MaxWalkSpeed` (* (`self.MaxWalkSpeed`) (`self.InBuildingPlayerAdjustmentsMultiplier`)))
      ;;;[1 0.5906 0.6308] Debug
      (`KismetSystemLibrary.PrintString` (`KismetStringLibrary.Concat_StrStr` "Movement Speed: " (`KismetStringLibrary.Conv_DoubleToString` (`self.MaxWalkSpeed`)))))
    (:`CastFailed`
      (`KismetSystemLibrary.PrintString` "Cast to BP_HouseExterior FAILED when trying to LEAVE the Trigger!"))))

(fn `UserConstructionScript`)