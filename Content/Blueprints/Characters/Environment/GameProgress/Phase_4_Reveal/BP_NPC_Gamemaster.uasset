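; BP_NPC_Gamemaster is a flipbook-animated NPC, filed under the Phase 4 reveal, that appears and vanishes based on player proximity.
; When a tagged BP_Player enters its InteractionRadius, the sprite plays an appear flipbook, then switches to idle after a fixed delay.
; When the player leaves, it plays a disappear flipbook and destroys itself after a delay, so it does not return.
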(event `self.InteractionRadius.OnComponentBeginOverlap`
  (params (OverlappedComponent :type "PrimitiveComponent Object Reference") (OtherActor :type "Actor Object Reference") (OtherComp :type "PrimitiveComponent Object Reference") (OtherBodyIndex :type Integer) (bFromSweep :type Boolean) (SweepResult :type "HitResult Structure (by ref)"))
  (bind _asbp_player (cast `/Game/Blueprints/Characters/BP_Player` OtherActor))
  (if (`self.ActorHasTag` _asbp_player "Player")
    (`PaperFlipbookComponent.SetFlipbook` (`self.Sprite`) "/Game/Assets/Sprites/Characters/Gamemaster/Animations/GM_appear.GM_appear")
    (`KismetSystemLibrary.Delay` 4.0)
    (`PaperFlipbookComponent.SetFlipbook` (`self.Sprite`) "/Game/Assets/Sprites/Characters/Gamemaster/Animations/GM_Idle.GM_Idle")))

(event `self.InteractionRadius.OnComponentEndOverlap`
  (params (OverlappedComponent :type "PrimitiveComponent Object Reference") (OtherActor :type "Actor Object Reference") (OtherComp :type "PrimitiveComponent Object Reference") (OtherBodyIndex :type Integer))
  (bind _asbp_player (cast `/Game/Blueprints/Characters/BP_Player` OtherActor))
  (if (`self.ActorHasTag` _asbp_player "Player")
    (`PaperFlipbookComponent.SetFlipbook` (`self.Sprite`) "/Game/Assets/Sprites/Characters/Gamemaster/Animations/GM_disappear.GM_disappear")
    (`KismetSystemLibrary.Delay` 3.0)
    (`self.K2_DestroyActor`)))

(fn `UserConstructionScript`
  (`parent.UserConstructionScript`))