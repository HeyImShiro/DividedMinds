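; BP_Bird is an ambient Paper2D bird that pecks in place until the player approaches, then flies away.
; BeginPlay picks a random color variant, whose index selects both the peck and fly flipbooks.
; When a Player-tagged actor overlaps TriggerRadius, it swaps to flying, plays a pitch-randomized sound and schedules its destruction.
; One of two timelines moves it diagonally upward, away from the player's side along X, and sets its facing.
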(event `self.ReceiveBeginPlay`
  (bind _peckvariants (`self.PeckVariants`))
  ;[1 1 1] Create Random Color Bird on game start
  (bind _output_get (set `self.ChosenRandomVariant` (`KismetMathLibrary.RandomInteger` (`KismetArrayLibrary.Array_Length` _peckvariants))))
  (`PaperFlipbookComponent.SetFlipbook` (`self.BirdBlue_peck`) (`|GetArrayItem` _peckvariants _output_get)))

(event `self.TriggerRadius.OnComponentBeginOverlap`
  (params (OverlappedComponent :type "PrimitiveComponent Object Reference") (OtherActor :type "Actor Object Reference") (OtherComp :type "PrimitiveComponent Object Reference") (OtherBodyIndex :type Integer) (bFromSweep :type Boolean) (SweepResult :type "HitResult Structure (by ref)"))
  (bind (_returnvalue_x _returnvalue_y _returnvalue_z) (`KismetMathLibrary.BreakVector` (`self.K2_GetActorLocation`)))
  (bind (_returnvalue_x_2 _returnvalue_y_2) (`KismetMathLibrary.BreakVector` (`self.K2_GetActorLocation`)))
  (bind (_returnvalue_x_3 _returnvalue_y_3 _returnvalue_z_2) (`KismetMathLibrary.BreakVector` (`self.K2_GetActorLocation`)))
  (bind (_returnvalue_x_4 _returnvalue_y_4) (`KismetMathLibrary.BreakVector` (`self.K2_GetActorLocation`)))
  (bind _returnvalue_x_5 (`KismetMathLibrary.BreakVector` (`self.K2_GetActorLocation`)))
  (bind _returnvalue_x_6 (`KismetMathLibrary.BreakVector` (`self.K2_GetActorLocation` OtherActor)))
  ;[1 1 1] Check if Player is close
  (if (`self.ActorHasTag` OtherActor "Player")
    (`PaperFlipbookComponent.SetFlipbook` (`self.BirdBlue_peck`) (`|GetArrayItem` (`self.FlyVariants`) (`self.ChosenRandomVariant`))) ; Change to flying animation
    (`GameplayStatics.PlaySound2D` "/Game/Assets/Audio/SoundCues/BirdsCue.BirdsCue" 0.5 (`KismetMathLibrary.RandomFloatInRange` 0.9 1.0) 0.0 null null false)
    (`|ExecutionSequence`
      (:`then_0`
        ;[1 1 1] Delete Bird after certain amount of time
        (`KismetSystemLibrary.Delay` 3.5)
        (`self.K2_DestroyActor`))
      (:`then_1`
        (if (> _returnvalue_x_6 _returnvalue_x_5)
          ;[1 1 1] fly away WEST
          (bind (_direction _upwardmovement) (`Timeline|Timeline`)
            (:`Update`
              (bind _returnvalue (* _upwardmovement 300.0))
              (`self.K2_SetActorLocation` (`KismetMathLibrary.MakeVector` (- _returnvalue_x_3 _returnvalue) _returnvalue_y_4 (+ _returnvalue _returnvalue_z_2)))
              (`self.K2_SetActorRotation` (struct :`Yaw` 180.0))))
          (else
            ;[1 1 1] fly away EAST
            (bind (_direction_2 _upwardmovement_2) (`Timeline|Timeline_0`)
              (:`Update`
                (bind _returnvalue_2 (* _upwardmovement_2 300.0))
                (`self.K2_SetActorLocation` (`KismetMathLibrary.MakeVector` (+ _returnvalue_x _returnvalue_2) _returnvalue_y_2 (+ _returnvalue_2 _returnvalue_z)))
                (`self.K2_SetActorRotation` (struct))))))))))

(fn `UserConstructionScript`)