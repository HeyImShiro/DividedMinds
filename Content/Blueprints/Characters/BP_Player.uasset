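; Player character for a 2D flipbook game, handling movement, sprinting, pause menu and NPC dialogue.
; Tick switches walk and idle animations, plays delayed biome-based footsteps and flips the sprite through control rotation.
; Capsule overlaps with tagged forest and house triggers set the biome.
; A chain of collapsed graphs applies or reverts house adjustments to camera, depth of field, sprite, speed and exterior visibility.
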(event `InputAction|Pause Game`
  (params (Key :type "Key Structure"))
  (bind _returnvalue (`GameplayStatics.GetPlayerController` 0))
  ;[1 1 1] Pause Game
  (:`Pressed`
    (if (not (`self.isPauseMenuOpen?`))
      (set `self.isPauseMenuOpen?` true)
      (bind _returnvalue_2 (`|CreateWidget` "/Game/Blueprints/UI/W_PauseMenu.W_PauseMenu_C" _returnvalue))
      (bind _output_get (set `self.PauseMenuWidget` _returnvalue_2))
      (`UserWidget.AddToViewport` _output_get 0)
      (`WidgetBlueprintLibrary.SetInputMode_UIOnlyEx` _returnvalue (`self.PauseMenuWidget`))
      (set `PlayerController.bShowMouseCursor` true (`GameplayStatics.GetPlayerController` 0))
      (`GameplayStatics.SetGamePaused` true)
      (else
        (set `self.isPauseMenuOpen?` false)
        (`Widget.RemoveFromParent` (`self.PauseMenuWidget`))
        (`GameplayStatics.SetGamePaused` false)
        (`WidgetBlueprintLibrary.SetInputMode_GameOnly` _returnvalue)
        (set `PlayerController.bShowMouseCursor` false (`GameplayStatics.GetPlayerController` 0))))))

(event `self.ReceiveBeginPlay`
  ;[1 1 1] Called at Game Start
)

(event `self.ReceiveTick`
  (params (DeltaSeconds :type "Float (single-precision)"))
  ;[1 1 1] Will be called every Frame
  ;;[1 1 1] Check if Animation needs to be changed
  (`self.UpdateAnimation`)
  ;;[1 1 1] Check if Player Sprite needs to be flipped
  (`self.UpdateControlRotation`))

(event `InputAxis|MoveRight`
  (params (AxisValue :type "Float (single-precision)"))
  ;[1 1 1] Move
  (if (`self.isSprinting?`)
    (set `CharacterMovementComponent.MaxWalkSpeed` (* (`self.MaxWalkSpeed`) (`self.SprintSpeedMultiplier`)) (`self.CharacterMovement`))
    (else
      (set `CharacterMovementComponent.MaxWalkSpeed` (`self.MaxWalkSpeed`) (`self.CharacterMovement`))))
  (`self.AddMovementInput` (1.0 0.0 0.0) AxisValue))

(event `InputAxis|MoveUp`
  (params (AxisValue :type "Float (single-precision)"))
  ;[1 1 1] Move
  (`self.AddMovementInput` (0.0 -1.0 0.0) (* AxisValue (`self.VerticalMovementSpeedMultiplier`))))

(event `Key|LeftShift`
  (params (Key :type "Key Structure"))
  ;[1 1 1] Move
  (:`Pressed`
    (set `self.isSprinting?` true)
    ;;[1 1 1] adjust footstep speed while sprinting
    (set `self.FootstepDelay` 0.3))
  (:`Released`
    (set `self.isSprinting?` false)
    (set `self.FootstepDelay` 0.4)))

(event `UpdateAnimation`
  (bind _returnvalue (`KismetMathLibrary.RandomFloatInRange` 0.9 1.1))
  (bind _sprite (`self.Sprite`))
  ;[1 1 1] Change Animation when running
  (if (> (`KismetMathLibrary.VSize` (`MovementComponent.Velocity` (`self.CharacterMovement`))) 0.0)
    (`PaperFlipbookComponent.SetFlipbook` _sprite "/Game/Assets/Sprites/Characters/Ku/WithNormals/walking/Ku_normals_walking.Ku_normals_walking")
    (set `self.isAbleToIdle?` true)
    (bind _output_get (set `self.isWalking?` true))
    ;[1 1 1] Footsteps
    (`KismetSystemLibrary.Delay` (`self.FootstepDelay`))
    (if _output_get
      (`/Engine/EditorBlueprintResources/StandardMacros.CompareInt` (`self.BiomeIndex`) 1
        (:`>`
          ;[0.1897 1 0] Footstep SFX depending on Biome: 0 = Bridge; 1 = Forest; 2 = House
          (`GameplayStatics.PlaySound2D` "/Game/Assets/Audio/SoundCues/FootstepCue_HouseFloor.FootstepCue_HouseFloor" 0.05 _returnvalue 0.0 null null false))
        (:`==`
          (`GameplayStatics.PlaySound2D` "/Game/Assets/Audio/SoundCues/FootstepCue_Dirt.FootstepCue_Dirt" 0.05 _returnvalue 0.0 null null false))
        (:`<`
          (`GameplayStatics.PlaySound2D` "/Game/Assets/Audio/SoundCues/FootstepCue_Asphalt.FootstepCue_Asphalt" 0.05 _returnvalue 0.0 null null))))
    (elif (`self.isAbleToIdle?`)
      (`PaperFlipbookComponent.SetFlipbook` _sprite "/Game/Assets/Sprites/Characters/Ku/WithNormals/idle/Ku_Normal_Idle.Ku_Normal_Idle")
      (set `self.isWalking?` false))))

(event `UpdateControlRotation`
  ;[1 1 1] Rotate Character to face the other side when walking in other direction
  (`/Engine/EditorBlueprintResources/StandardMacros.IsValid` (`self.GetController`)
    (:`Is Valid`
      (`/Engine/EditorBlueprintResources/StandardMacros.CompareFloat` (.x (`MovementComponent.Velocity` (`self.CharacterMovement`)))
        (:`>`
          (`Controller.SetControlRotation` (`self.GetController`) (`KismetMathLibrary.MakeRotator` 0.0 0.0 180.0)))
        (:`<`
          (`Controller.SetControlRotation` (`self.GetController`) (`KismetMathLibrary.MakeRotator` 0.0)))))))

(event `Key|F`
  (params (Key :type "Key Structure"))
  ;[1 1 1] Play Animation on F
  (:`Pressed`
    (if (`self.isAbleToIdle?`)
      (set `self.isAbleToIdle?` false)
      (else
        (set `self.isAbleToIdle?` true)))
    (`/Engine/EditorBlueprintResources/StandardMacros.IsValid` (`self.GetController`)
      (:`Is Valid`
        (`/Engine/EditorBlueprintResources/StandardMacros.CompareFloat` (.x (`MovementComponent.Velocity` (`self.CharacterMovement`)))
          (:`==`
            (`PaperFlipbookComponent.SetFlipbook` (`self.Sprite`) "/Game/Assets/Sprites/Characters/Ku/WithNormals/thinking/Ku_normals_thinking.Ku_normals_thinking")))))))

(event `Key|R`
  (params (Key :type "Key Structure"))
  ;[1 0 0] DEBUG TOOL: TIME SPEEDUP
  (:`Pressed`
    (`GameplayStatics.SetGlobalTimeDilation` 3.0))
  (:`Released`
    (`GameplayStatics.SetGlobalTimeDilation` 1.0)))

(event `self.CapsuleComponent.OnComponentBeginOverlap`
  (params (OverlappedComponent :type "PrimitiveComponent Object Reference") (OtherActor :type "Actor Object Reference") (OtherComp :type "PrimitiveComponent Object Reference") (OtherBodyIndex :type Integer) (bFromSweep :type Boolean) (SweepResult :type "HitResult Structure (by ref)"))
  (bind _springarm (`self.SpringArm`))
  (bind _sprite (`self.Sprite`))
  (bind ((`AutoExposureMethod` _autoexposuremethod) (`AmbientCubemapTint` _ambientcubemaptint) (`AmbientCubemapIntensity` _ambientcubemapintensity) (`AmbientCubemap` _ambientcubemap) (`DepthOfFieldFstop` _depthoffieldfstop) (`DepthOfFieldMinFstop` _depthoffieldminfstop) (`DepthOfFieldBladeCount` _depthoffieldbladecount) (`AutoExposureBias` _autoexposurebias) (`AutoExposureMaxBrightness` _autoexposuremaxbrightness) (`VignetteIntensity` _vignetteintensity) (`DepthOfFieldSensorWidth` _depthoffieldsensorwidth) (`DepthOfFieldSqueezeFactor` _depthoffieldsqueezefactor) (`DepthOfFieldFocalDistance` _depthoffieldfocaldistance) (`DepthOfFieldVignetteSize` _depthoffieldvignettesize)) (break `PostProcessSettings` (`CameraComponent.PostProcessSettings` (`self.Camera`))))
  ;[1 1 1] VISUAL CHANGES WHEN ENTERING HOUSE
  (`|ExecutionSequence`
    (:`then_0`
      (bind _asbp_forest_biome (cast `/Game/Blueprints/Environment/BP_ForestBiome` OtherActor))
      (if (`self.ActorHasTag` _asbp_forest_biome "ForestBiome")
        (set `self.BiomeIndex` 1)
        (`KismetSystemLibrary.PrintString` "Biome: 1 ; Forest" true true (struct :`R` 0.147027 :`G` 1.0 :`B` 0.184475 :`A` 1.0))
        (else
          (`KismetSystemLibrary.PrintString` "Trigger does not have ForestBiome Tag!"))))
    (:`then_1`
      ;;[1 1 1] Adjustments When entering/leaving House
      (bind _asbp_house_exterior (cast `/Game/Blueprints/Environment/BP_HouseExterior` OtherActor))
      (if (`self.ActorHasTag` _asbp_house_exterior "HouseTrigger")
        (set `self.BiomeIndex` 2)
        (`KismetSystemLibrary.PrintString` "Biome: 2 ; House" true true (struct :`R` 0.147027 :`G` 1.0 :`B` 0.184475 :`A` 1.0))
        (set `SpringArmComponent.TargetArmLength` (/ (`SpringArmComponent.TargetArmLength` _springarm) (`self.InBuildingPlayerAdjustmentsMultiplier`)) _springarm)
        (`SceneComponent.SetWorldScale3D` _sprite (/ (`SceneComponent.K2_GetComponentScale` _sprite) (`self.InBuildingPlayerAdjustmentsMultiplier`)))
        (`SceneComponent.K2_AddLocalOffset` (`self.Sprite`) (0.0 0.0 -11.5) false false)
        (bind _asbp_house_exterior_2 (cast `/Game/Blueprints/Environment/BP_HouseExterior` OtherActor)
          (:`then`
            (`SceneComponent.SetVisibility` (`/Game/Blueprints/Environment/BP_HouseExterior.StaticMesh` _asbp_house_exterior_2) false true)
            (set `CameraComponent.PostProcessSettings` (make `PostProcessSettings` :`AutoExposureMethod` _autoexposuremethod :`AmbientCubemapTint` _ambientcubemaptint :`AmbientCubemapIntensity` _ambientcubemapintensity :`AmbientCubemap` _ambientcubemap :`DepthOfFieldFstop` _depthoffieldfstop :`DepthOfFieldMinFstop` _depthoffieldminfstop :`DepthOfFieldBladeCount` _depthoffieldbladecount :`AutoExposureBias` _autoexposurebias :`AutoExposureMaxBrightness` _autoexposuremaxbrightness :`VignetteIntensity` 0.75 :`DepthOfFieldSensorWidth` _depthoffieldsensorwidth :`DepthOfFieldSqueezeFactor` _depthoffieldsqueezefactor :`DepthOfFieldFocalDistance` 360.0 :`DepthOfFieldVignetteSize` _depthoffieldvignettesize) (`self.Camera`))
            (set `self.MaxWalkSpeed` (/ (`self.MaxWalkSpeed`) (`self.InBuildingPlayerAdjustmentsMultiplier`)))
            (`GameplayStatics.PlaySound2D` "/Game/Assets/Audio/SFX/15419__pagancow__dorm-door-opening.15419__pagancow__dorm-door-opening" 0.5 (`KismetMathLibrary.RandomFloatInRange` 1.05 1.1) 0.8 null null))
          (:`CastFailed`
            (`KismetSystemLibrary.PrintString` "Cast to BP_HouseExterior FAILED when trying to ENTER  the Trigger!")))
        (else
          (`KismetSystemLibrary.PrintString` "HouseTrigger is not correctly Tagged!" :!label _label))))))

(event `self.CapsuleComponent.OnComponentEndOverlap`
  (params (OverlappedComponent :type "PrimitiveComponent Object Reference") (OtherActor :type "Actor Object Reference") (OtherComp :type "PrimitiveComponent Object Reference") (OtherBodyIndex :type Integer))
  (bind _springarm (`self.SpringArm`))
  (bind _sprite (`self.Sprite`))
  (bind ((`AutoExposureMethod` _autoexposuremethod) (`AmbientCubemapTint` _ambientcubemaptint) (`AmbientCubemapIntensity` _ambientcubemapintensity) (`AmbientCubemap` _ambientcubemap) (`DepthOfFieldFstop` _depthoffieldfstop) (`DepthOfFieldMinFstop` _depthoffieldminfstop) (`DepthOfFieldBladeCount` _depthoffieldbladecount) (`AutoExposureBias` _autoexposurebias) (`AutoExposureMaxBrightness` _autoexposuremaxbrightness) (`VignetteIntensity` _vignetteintensity) (`DepthOfFieldSensorWidth` _depthoffieldsensorwidth) (`DepthOfFieldSqueezeFactor` _depthoffieldsqueezefactor) (`DepthOfFieldFocalDistance` _depthoffieldfocaldistance) (`DepthOfFieldVignetteSize` _depthoffieldvignettesize)) (break `PostProcessSettings` (`CameraComponent.PostProcessSettings` (`self.Camera`))))
  ;[1 1 1] VISUAL CHANGES WHEN ENTERING HOUSE
  (`|ExecutionSequence`
    (:`then_0`
      (bind _asbp_forest_biome (cast `/Game/Blueprints/Environment/BP_ForestBiome` OtherActor)
        (:`then`
          (if (`self.ActorHasTag` _asbp_forest_biome "ForestBiome")
            (set `self.BiomeIndex` 0)
            (`KismetSystemLibrary.PrintString` "Biome: 0 ; Bridge" true true (struct :`R` 0.147027 :`G` 1.0 :`B` 0.184475 :`A` 1.0))
            (else
              (`KismetSystemLibrary.PrintString` "Player has left a trigger that is NOT ForestBiome"))))
        (:`CastFailed`
          (`KismetSystemLibrary.PrintString` "Failed cast to BP_ForestBiome in \"Change to Bridge Biome\" withing BP_Player!"))))
    (:`then_1`
      ;;[1 1 1] Adjustments When entering/leaving House
      (bind _asbp_house_exterior (cast `/Game/Blueprints/Environment/BP_HouseExterior` OtherActor))
      (if (`self.ActorHasTag` _asbp_house_exterior "HouseTrigger")
        (`KismetSystemLibrary.PrintString` "Player LEFT HouseTrigger")
        (set `SpringArmComponent.TargetArmLength` (* (`SpringArmComponent.TargetArmLength` _springarm) (`self.InBuildingPlayerAdjustmentsMultiplier`)) _springarm)
        (`SceneComponent.SetWorldScale3D` _sprite (* (`self.InBuildingPlayerAdjustmentsMultiplier`) (`SceneComponent.K2_GetComponentScale` _sprite)))
        (`SceneComponent.K2_AddLocalOffset` (`self.Sprite`) (0.0 0.0 11.5) false false)
        (bind _asbp_house_exterior_2 (cast `/Game/Blueprints/Environment/BP_HouseExterior` OtherActor)
          (:`then`
            (`SceneComponent.SetVisibility` (`/Game/Blueprints/Environment/BP_HouseExterior.StaticMesh` _asbp_house_exterior_2) true true)
            (set `CameraComponent.PostProcessSettings` (make `PostProcessSettings` :`AutoExposureMethod` _autoexposuremethod :`AmbientCubemapTint` _ambientcubemaptint :`AmbientCubemapIntensity` _ambientcubemapintensity :`AmbientCubemap` _ambientcubemap :`DepthOfFieldFstop` 1.2 :`DepthOfFieldMinFstop` 0.0 :`AutoExposureBias` _autoexposurebias :`AutoExposureMaxBrightness` _autoexposuremaxbrightness :`DepthOfFieldSensorWidth` 200.0 :`DepthOfFieldFocalDistance` 520.0 :`DepthOfFieldVignetteSize` _depthoffieldvignettesize) (`self.Camera`))
            (set `self.MaxWalkSpeed` (* (`self.MaxWalkSpeed`) (`self.InBuildingPlayerAdjustmentsMultiplier`)))
            (`GameplayStatics.PlaySound2D` "/Game/Assets/Audio/SFX/15419__pagancow__dorm-door-opening.15419__pagancow__dorm-door-opening" 0.5 (`KismetMathLibrary.RandomFloatInRange` 0.9 0.95) 0.8 null null))
          (:`CastFailed`
            (`KismetSystemLibrary.PrintString` "Cast to BP_HouseExterior FAILED when trying to LEAVE the Trigger!")))
        (else
          (goto _label))))))

(event `InputAction|Interact`
  (params (Key :type "Key Structure"))
  (bind _maininterfacereference (`self.MainInterfaceReference`))
  (bind _maininterfacereference_2 (`self.MainInterfaceReference`))
  ;[1 1 1] Interact / Dialogue
  (:`Pressed`
    (if (`self.isInInteractionRange?`)
      (if (`self.isDialogueOpen?`)
        (bind _asw_dialogue_interface (cast `/Game/Blueprints/UI/W_DialogueInterface` _maininterfacereference)
          (:`then`
            (if (`/Game/Blueprints/UI/W_DialogueInterface.isDialogueExhausted?` _asw_dialogue_interface)
              (`/Game/Blueprints/UI/W_DialogueInterface.CloseDialogue` _maininterfacereference_2)
              (set `self.isDialogueOpen?` false)
              (`KismetSystemLibrary.PrintString` "Dialogue closed!")
              (set `self.MaxWalkSpeed` 150.0)
              (else
                (`/Game/Blueprints/UI/W_DialogueInterface.AdvanceDialogue` _maininterfacereference_2))))
          (:`CastFailed`
            (`KismetSystemLibrary.PrintString` "Cast to W_MainInterfaceWidget failed in BP_Player! ")))
        (else
          (bind _returnvalue (`|CreateWidget` "/Game/Blueprints/UI/W_DialogueInterface.W_DialogueInterface_C"))
          (`UserWidget.AddToViewport` _returnvalue 0)
          (set `self.MainInterfaceReference` _returnvalue)
          (bind (_name _currentstate _portrait _dialoguearray) (break `/Game/Blueprints/Characters/S_CharacterStructure` (stale `PassNPCInfo` CharacterInfo)))
          (`/Game/Blueprints/UI/W_DialogueInterface.OpenDialogue` _maininterfacereference _name _portrait _dialoguearray)
          (set `self.isDialogueOpen?` true)
          (`KismetSystemLibrary.PrintString` "Dialogue opened!")
          (set `self.MaxWalkSpeed` 0.0))))))

(event `PassNPCInfo`
  (params (CharacterInfo :type "/Game/Blueprints/Characters/S_CharacterStructure Structure"))
  ;[1 1 1] Interact / Dialogue
)

(fn `UserConstructionScript`)