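; BP_NPC_Master is an NPC Blueprint that tells the player when it is within interaction range.
; Begin and end overlaps on InteractionRadius cast the other actor to BP_Player, check its Player tag, and set IsInInteractionRange on it.
; Entering also passes this NPC's CharacterInfo to the player through PassNPCInfo.
; A BP_Player without the tag triggers a debug print.
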(event `self.InteractionRadius.OnComponentBeginOverlap`
  (params (OverlappedComponent :type "PrimitiveComponent Object Reference") (OtherActor :type "Actor Object Reference") (OtherComp :type "PrimitiveComponent Object Reference") (OtherBodyIndex :type Integer) (bFromSweep :type Boolean) (SweepResult :type "HitResult Structure (by ref)"))
  ;[1 1 1] Check if Overlapped with Player Character
  (bind _asbp_player (cast `/Game/Blueprints/Characters/BP_Player` OtherActor))
  (if (`self.ActorHasTag` _asbp_player "Player")
    ;[1 1 1] Set Variable in Player BP
    (set `/Game/Blueprints/Characters/BP_Player.isInInteractionRange?` true _asbp_player)
    (`/Game/Blueprints/Characters/BP_Player.PassNPCInfo` _asbp_player (`self.CharacterInfo`)) ; Send NPC Info to Player BP
    (else
      ;[1 0.5976 0.2779] DEBUG messages
      (`KismetSystemLibrary.PrintString` "Other Actor is not tagged as Player!" :!label _label))))

(event `self.InteractionRadius.OnComponentEndOverlap`
  (params (OverlappedComponent :type "PrimitiveComponent Object Reference") (OtherActor :type "Actor Object Reference") (OtherComp :type "PrimitiveComponent Object Reference") (OtherBodyIndex :type Integer))
  ;[1 1 1] Check if Overlapped with Player Character
  (bind _asbp_player (cast `/Game/Blueprints/Characters/BP_Player` OtherActor))
  (if (`self.ActorHasTag` _asbp_player "Player")
    ;[1 1 1] Set Variable in Player BP
    (set `/Game/Blueprints/Characters/BP_Player.isInInteractionRange?` false _asbp_player)
    (else
      (goto _label))))

(fn `UserConstructionScript`)