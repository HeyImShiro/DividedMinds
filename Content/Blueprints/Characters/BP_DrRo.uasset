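; BP_DrRo is the Dr. Ro character, which the player can interact with inside an InteractionRadius.
; Overlap by a BP_Player tagged "Player" toggles input on the actor and sets the player's IsInInteractionRange flag.
; While input is enabled, pressing E casts the overlapping actor to BP_Player and passes CharacterInfo to its InteractEvent.
; CharacterState only selects a debug message at BeginPlay.
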(event `self.ReceiveBeginPlay`
  (switch `/Game/Blueprints/Characters/E_NPC_States` (`self.CharacterState`)
    (:`NewEnumerator0`
      (`KismetSystemLibrary.PrintString` "Dr.Ro is walking!"))
    (:`NewEnumerator1`
      (`KismetSystemLibrary.PrintString` "Dr.Ro is talking!"))
    (:`NewEnumerator2`
      (`KismetSystemLibrary.PrintString` "Dr.Ro is idle!"))))

(event `Key|E`
  (params (Key :type "Key Structure"))
  (:`Pressed`
    (`KismetSystemLibrary.PrintString` "pressed E!")
    (bind _asbp_player (cast `/Game/Blueprints/Characters/BP_Player` (stale `self.InteractionRadius.OnComponentBeginOverlap` OtherActor))
      (:`then`
        (`/Game/Blueprints/Characters/BP_Player.InteractEvent` _asbp_player (`self.CharacterInfo`)))
      (:`CastFailed`
        (`KismetSystemLibrary.PrintString` "Cast to BP_Player failed!")))))

(event `self.InteractionRadius.OnComponentBeginOverlap`
  (params (OverlappedComponent :type "PrimitiveComponent Object Reference") (OtherActor :type "Actor Object Reference") (OtherComp :type "PrimitiveComponent Object Reference") (OtherBodyIndex :type Integer) (bFromSweep :type Boolean) (SweepResult :type "HitResult Structure (by ref)"))
  (bind _asbp_player (cast `/Game/Blueprints/Characters/BP_Player` OtherActor)
    (:`then`
      (if (`self.ActorHasTag` _asbp_player "Player")
        (`self.EnableInput` (`GameplayStatics.GetPlayerController` 0))
        (`KismetSystemLibrary.PrintString` "Player ENTERED InteractionRadius!")
        (set `/Game/Blueprints/Characters/BP_Player.isInInteractionRange?` true _asbp_player)
        (else
          (`KismetSystemLibrary.PrintString` "Other Actor is not tagged as Player!" :!label _label))))
    (:`CastFailed`
      (`KismetSystemLibrary.PrintString` "Cast to BP_Player has failed!" :!label _label_2))))

(event `self.InteractionRadius.OnComponentEndOverlap`
  (params (OverlappedComponent :type "PrimitiveComponent Object Reference") (OtherActor :type "Actor Object Reference") (OtherComp :type "PrimitiveComponent Object Reference") (OtherBodyIndex :type Integer))
  (bind _asbp_player (cast `/Game/Blueprints/Characters/BP_Player` OtherActor)
    (:`then`
      (if (`self.ActorHasTag` _asbp_player "Player")
        (`self.DisableInput` (`GameplayStatics.GetPlayerController` 0))
        (`KismetSystemLibrary.PrintString` "Player LEFT InteractionRadius!")
        (set `/Game/Blueprints/Characters/BP_Player.isInInteractionRange?` false _asbp_player)
        (else
          (goto _label))))
    (:`CastFailed`
      (goto _label_2))))

(fn `UserConstructionScript`)