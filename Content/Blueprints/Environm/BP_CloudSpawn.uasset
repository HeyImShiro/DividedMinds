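; Cloud spawner actor that spawns a BP_Cloud on BeginPlay and then keeps spawning more at a set interval.
; Tick feeds a Delay of SpawnInterval back into the spawn node, acting as a repeating timer.
; Each cloud's transform derives from the spawner's, with a positive random location offset (halved in height), randomized yaw and random per-axis scale added.
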(event `self.ReceiveBeginPlay`
  (bind _returnvalue (`self.GetTransform`))
  (bind _spawnlocationvariance (`self.SpawnLocationVariance`))
  (bind _maximumsize (`self.MaximumSize`))
  (bind _minimumsize (`self.MinimumSize`))
  (bind (_returnvalue_x _returnvalue_y _returnvalue_z) (`KismetMathLibrary.BreakVector` (`KismetMathLibrary.MakeVector` (`KismetMathLibrary.RandomFloatInRange` _minimumsize _maximumsize) (`KismetMathLibrary.RandomFloatInRange` _minimumsize _maximumsize) (`KismetMathLibrary.RandomFloatInRange` _minimumsize _maximumsize))))
  (bind (_returnvalue_x_2 _returnvalue_y_2 _returnvalue_z_2) (`KismetMathLibrary.BreakVector` (`KismetMathLibrary.MakeVector` (`KismetMathLibrary.RandomFloatInRange` 0.0 _spawnlocationvariance) (`KismetMathLibrary.RandomFloatInRange` 0.0 _spawnlocationvariance) (* (`KismetMathLibrary.RandomFloatInRange` 0.0 _spawnlocationvariance) 0.5))))
  ;[1 1 1] Spawn Cloud on Game Start and then keep spawning Clouds every X seconds
  (`|SpawnActorFromClass` "/Game/Blueprints/Environm/BP_Cloud.BP_Cloud_C" (`KismetMathLibrary.MakeTransform` (`KismetMathLibrary.MakeVector` (+ _returnvalue_x_2 (.x (.location _returnvalue))) (+ _returnvalue_y_2 (.y (.location _returnvalue))) (+ _returnvalue_z_2 (.z (.location _returnvalue)))) (`KismetMathLibrary.MakeRotator` (.roll (.rotation _returnvalue)) (.pitch (.rotation _returnvalue)) (`KismetMathLibrary.RandomFloatInRange` (.yaw (.rotation _returnvalue)) 360.0)) (`KismetMathLibrary.MakeVector` (+ (.x (.scale _returnvalue)) _returnvalue_x) (+ (.y (.scale _returnvalue)) _returnvalue_y) (+ (.z (.scale _returnvalue)) _returnvalue_z))) "Undefined" "MultiplyWithRoot" null null :!label _label))

(event `self.ReceiveTick`
  (params (DeltaSeconds :type "Float (single-precision)"))
  ;[1 1 1] Spawn Cloud on Game Start and then keep spawning Clouds every X seconds
  (`KismetSystemLibrary.Delay` (`self.SpawnInterval`))
  (goto _label))

(fn `UserConstructionScript`)