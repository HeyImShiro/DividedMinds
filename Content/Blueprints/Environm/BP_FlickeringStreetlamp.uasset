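; Streetlamp Blueprint that switches its lights off while the player is inside its trigger box and back on when they leave.
; Box overlap events filter for a BP_Player tagged "Player", then set SpotLight and PointLight intensities, flipping a LightsOn bool each time.
; BeginPlay zeroes the mesh material's emissive boost and initializes LightsOn.
; Despite the asset name, the graphs contain no flicker logic.
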(event `self.ReceiveBeginPlay`
  ;[1 1 1] Turn off Emission on MaterialInstance
  (`MeshComponent.SetScalarParameterValueOnMaterials` (`self.StaticMesh`) "Emissive Boost Multiplier" 0.0)
  ;[1 1 1] Initialize Bool on Start
  (set `self.LightsOn` true))

(event `self.Box.OnComponentBeginOverlap`
  (params (OverlappedComponent :type "PrimitiveComponent Object Reference") (OtherActor :type "Actor Object Reference") (OtherComp :type "PrimitiveComponent Object Reference") (OtherBodyIndex :type Integer) (bFromSweep :type Boolean) (SweepResult :type "HitResult Structure (by ref)"))
  ;[1 1 1] Check if it's the Player
  (bind _asbp_player (cast `/Game/Blueprints/Chars/BP_Player` OtherActor))
  (if (`self.ActorHasTag` _asbp_player "Player")
    (`LightComponent.SetIntensity` (`self.SpotLight`) 0.0)
    (`LightComponent.SetIntensity` (`self.PointLight`) 0.0)
    (`ActorComponent.SetActive` (`self.DefaultSceneRoot`) false false)
    (if (`self.LightsOn`)
      (set `self.LightsOn` false)
      (else
        (set `self.LightsOn` true)))
    (else
      (`KismetSystemLibrary.PrintString` "Something that isn't tagged as Player has ENTERED the house!" :!label _label))))

(event `self.Box.OnComponentEndOverlap`
  (params (OverlappedComponent :type "PrimitiveComponent Object Reference") (OtherActor :type "Actor Object Reference") (OtherComp :type "PrimitiveComponent Object Reference") (OtherBodyIndex :type Integer))
  ;[1 1 1] Check if it's the Player
  (bind _asbp_player (cast `/Game/Blueprints/Chars/BP_Player` OtherActor))
  (if (`self.ActorHasTag` _asbp_player "Player")
    (`LightComponent.SetIntensity` (`self.SpotLight`) 8.0)
    (`LightComponent.SetIntensity` (`self.PointLight`) 3.0)
    (if (`self.LightsOn`)
      (set `self.LightsOn` false)
      (else
        (set `self.LightsOn` true)))
    (else
      (goto _label))))

(fn `UserConstructionScript`)